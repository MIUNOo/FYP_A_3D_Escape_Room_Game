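; BP_TriggerLogic is a key-activated trigger volume that fires an action on another object.
; When an actor begins overlapping BoxTrigger, it checks that TriggerObject and Key are valid and that the actor is Key.
; It then calls OnTrigger on TriggerObject through the BPI_TriggerObject interface, keeping the trigger independent of the target's class.
; BeginPlay holds only an empty branch.
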(event OnComponentBeginOverlap(BoxTrigger)
  (params (OverlappedComponent :type Primitive%20Component%20Object%20Reference) (OtherActor :type Actor%20Object%20Reference) (OtherComp :type Primitive%20Component%20Object%20Reference) (OtherBodyIndex :type Integer) (bFromSweep :type Boolean) (SweepResult :type Hit%20Result%20Structure%20%28by%20ref%29))
  (if (and (Utilities|IsValid (Variables|Default|GetTriggerObject)) (Utilities|IsValid (Variables|Default|GetKey)))
    (if (== OtherActor (Variables|Default|GetKey))
      (bind _asbpi_trigger_object (Utilities|Casting|CastToBPI_TriggerObject (Variables|Default|GetTriggerObject)))
      (Default|OnTrigger _asbpi_trigger_object))))

(event EventBeginPlay
  (if true
    _))

(event Collision|EventActorBeginOverlap
  (params (OtherActor :type Actor%20Object%20Reference)))

(event EventTick
  (params (DeltaSeconds :type Float%20%28single-precision%29)))

(fn ConstructionScript)