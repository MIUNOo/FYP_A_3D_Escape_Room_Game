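; Interactable keypad lock that messages a linked TriggerObject when the player enters the correct KeypadCode.
; Interacting disables movement, hides the HUD, blends to the keypad camera with mouse clicks enabled, and binds a lock-leave event that restores player view.
; BP_KeypadButton child actors receive a parent reference for ButtonClicked input, shown in a code-length sliding window padded with underscores.
; Confirm shows success or error text, exiting to player view only on success.
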(event Custom|ButtonClicked
  (params (InputCode :type String) (IsConfirm :type Boolean) (IsReturn :type Boolean))
  (bind _inputedcode (Variables|Default|GetInputedCode))
  (bind _keypad_code (Variables|Default|GetKeypad%20Code))
  (bind _returnvalue (Utilities|String|Len _keypad_code))
  (bind _text (Variables|/Script/Engine.TextRenderComponent|GetText _inputedcode))
  (bind _returnvalue_2 (Utilities|String|ToString(Text) _text))
  (Variables|Default|SetIs%20Entering true)
  (if IsConfirm
    (CallFunction|Confirm)
    (else
      (if IsReturn
        (CallFunction|Backspace)
        (else
          ;[1 1 1] Append input code to current code and constraint it to code length
          (Variables|Default|SetCan%20Enter false)
          (Rendering|Components|TextRender|SetText _inputedcode (Utilities|Text|ToText(String) (Utilities|String|Append _returnvalue_2 InputCode)))
          (Rendering|Components|TextRender|SetText _inputedcode (Utilities|Text|ToText(String) (Utilities|String|GetSubstring _returnvalue_2 (- (Utilities|String|Len _returnvalue_2) _returnvalue) _returnvalue)))
          (Rendering|Components|TextRender|SetTextRenderColor _inputedcode (Math|Color|MakeColor 0 0 255 255))))
      (Variables|Default|SetIs%20Entering false)
      (Variables|Default|SetCan%20Enter true))))

(event Custom|Backspace
  (bind _inputedcode (Variables|Default|GetInputedCode))
  (bind _text (Variables|/Script/Engine.TextRenderComponent|GetText _inputedcode))
  (bind _returnvalue (Utilities|String|ToString(Text) _text))
  ;[1 1 1] Use substring to delete input code when clicking return button
  (Rendering|Components|TextRender|SetText (Variables|Default|GetInputedCode) (Utilities|Text|ToText(String) (Utilities|String|Append "_" (Utilities|String|GetSubstring _returnvalue 0 (- (Utilities|String|Len _returnvalue) 1))))))

(event Custom|Confirm
  (bind _inputedcode (Variables|Default|GetInputedCode))
  (bind _inputedcode_2 (Variables|Default|GetInputedCode))
  (bind _trigger_object (Variables|Default|GetTrigger%20Object))
  (if (Utilities|Enum|Equal(Enum) (Utilities|String|ToString(Text) (Variables|/Script/Engine.TextRenderComponent|GetText (Variables|Default|GetInputedCode))) (Variables|Default|GetKeypad%20Code))
    (Rendering|Components|TextRender|SetText _inputedcode_2 (Utilities|Text|MakeLiteralText "UNLOCKED!"))
    (Rendering|Components|TextRender|SetTextRenderColor _inputedcode_2 (Math|Color|MakeColor 0 255 0 255))
    (Variables|Default|SetCan%20Enter false)
    (Utilities|FlowControl|RetriggerableDelay 0.8)
    (CallFunction|ChangetoPlayerView)
    (Rendering|Components|TextRender|SetText (Variables|Default|GetInputedCode) (Utilities|Text|MakeLiteralText ""))
    (Utilities|IsValid _trigger_object
      (:Is%20Valid
        (Class|BPITriggerObject|OnTrigger(Message) _trigger_object)
        (CallFunction|UnbindEvents)))
    (else
      (Rendering|Components|TextRender|SetText _inputedcode (Utilities|Text|MakeLiteralText "WRONG CODE!!"))
      (Variables|Default|SetCan%20Enter false)
      (Utilities|FlowControl|RetriggerableDelay 0.8)
      (Rendering|Components|TextRender|SetText _inputedcode (Utilities|Text|MakeLiteralText (Utilities|Text|ToText(String) (Utilities|String|GetSubstring (Utilities|String|MakeLiteralString "____________________") 0 (Utilities|String|Len (Variables|Default|GetKeypad%20Code))))))
      (Rendering|Components|TextRender|SetTextRenderColor _inputedcode (Math|Color|MakeColor 0 0 255 127))
      (Variables|Default|SetCan%20Enter true)
      (Variables|Default|SetIs%20Entering false))))

(event Custom|UnbindEvents
  (bind _ac (Class|BPILockInterface|GetActorComponent(Message) (Game|GetPlayerController 0)))
  (EventDispatchers|UnbindallEventsfromLockLeave _ac))

(event Custom|Transition%20Back%20to%20Player
  (CallFunction|ChangetoPlayerView)
  (Variables|Default|SetIs%20Entering false)
  (Variables|Default|SetCan%20Enter true))

(event Custom|BindEvents
  (bind _ac (Class|BPILockInterface|GetActorComponent(Message) (Game|GetPlayerController 0)))
  (EventDispatchers|BindEventtoLockLeave _ac (delegate Custom|Transition%20Back%20to%20Player)))

(event EventBeginPlay
  (if (not (Utilities|Array|IsEmpty (Variables|Default|GetKeypad%20Code)))
    (Variables|Default|SetCan%20Enter true)
    (Variables|Default|SetIs%20Entering false)))

(fn ConstructionScript)

(fn ChangetoPlayerView
  (bind _returnvalue (Game|GetPlayerController 0))
  (bind _output_get (Variables|/Script/Engine.PlayerController|SetbShowMouseCursor _returnvalue false))
  (bind _output_get_2 (Variables|/Script/Engine.PlayerController|SetbEnableClickEvents _returnvalue _output_get))
  (Variables|/Script/Engine.PlayerController|SetbEnableMouseOverEvents _returnvalue _output_get_2)
  (Widget|SetVisibility (Variables|/Game/FirstPerson/Blueprints/BP_FirstPersonCharacter.BP_FirstPersonCharacter_C|GetHeadsUpDisplay (Variables|Default|GetInteractor)) "Visible")
  (Game|Player|SetViewTargetwithBlend (Game|GetPlayerController 0) (Components|GetOwner (Variables|/Game/FirstPerson/Blueprints/BP_FirstPersonCharacter.BP_FirstPersonCharacter_C|GetFirstPersonCamera (.AsBP%20First%20Person%20Character (Utilities|Casting|CastToBP_FirstPersonCharacter (Game|Player|GetPlayerPawn 0))))) 0.4 "VTBlend_Linear" 0.0 false)
  (Input|SetInputModeGameOnly (Game|GetPlayerController 0) false)
  (bind _ac (Class|BPILockInterface|GetActorComponent(Message) (Game|GetPlayerController 0)))
  (EventDispatchers|UnbindallEventsfromLockLeave _ac)
  (Pawn|Components|CharacterMovement|SetMovementMode (Variables|/Script/Engine.Character|GetCharacterMovement (Variables|Default|GetInteractor)) "MOVE_Walking" 0))

(fn Interactwith
  (params (Interactor :type BP%20First%20Person%20Character%20Object%20Reference) (HitComponent :type Primitive%20Component%20Object%20Reference))
  (bind _returnvalue (Game|GetPlayerController 0))
  (bind _inputedcode (Variables|Default|GetInputedCode))
  (if (Variables|Default|GetCan%20Enter)
    (CallFunction|BindEvents)
    (bind _output_get (Variables|Default|SetInteractor Interactor))
    (Pawn|Components|CharacterMovement|DisableMovement (Variables|/Script/Engine.Character|GetCharacterMovement _output_get))
    (Widget|SetVisibility (Variables|/Game/FirstPerson/Blueprints/BP_FirstPersonCharacter.BP_FirstPersonCharacter_C|GetHeadsUpDisplay _output_get) "Hidden")
    (Game|Player|SetViewTargetwithBlend (Game|GetPlayerController 0) (Components|GetOwner (Variables|Default|GetCamera)) 0.4 "VTBlend_Linear" 0.0 false)
    (bind _output_get_2 (Variables|/Script/Engine.PlayerController|SetbShowMouseCursor _returnvalue true))
    (bind _output_get_3 (Variables|/Script/Engine.PlayerController|SetbEnableClickEvents _returnvalue _output_get_2))
    (Variables|/Script/Engine.PlayerController|SetbEnableMouseOverEvents _returnvalue _output_get_3)
    (if (Utilities|Array|IsEmpty (Variables|Default|GetButtonsArray))
      (Rendering|Components|TextRender|SetText _inputedcode (Utilities|Text|MakeLiteralText (Utilities|Text|ToText(String) (Utilities|String|GetSubstring (Utilities|String|MakeLiteralString "____________________") 0 (Utilities|String|Len (Variables|Default|GetKeypad%20Code))))))
      (Rendering|Components|TextRender|SetTextRenderColor _inputedcode (Math|Color|MakeColor 0 0 255 127))
      (bind _output_get_4 (Variables|Default|SetButtonsArray (Utilities|Array|MakeArray (Variables|Default|GetButton0) (Variables|Default|GetButton1) (Variables|Default|GetButton2) (Variables|Default|GetButton3) (Variables|Default|GetButton4) (Variables|Default|GetButton5) (Variables|Default|GetButton6) (Variables|Default|GetButton7) (Variables|Default|GetButton8) (Variables|Default|GetButton9) (Variables|Default|GetButtonConfirm) (Variables|Default|GetButtonReturn))))
      (for _array_element _output_get_4
        (bind _asbp_keypad_button (Utilities|Casting|CastToBP_KeypadButton (Variables|/Script/Engine.ChildActorComponent|GetChildActor _array_element)))
        (Variables|/Game/Obj_OperatingObjects/BP_KeypadButton.BP_KeypadButton_C|SetKeypadParent _asbp_keypad_button self)))
    (Input|SetInputModeGameandUI (Game|GetPlayerController 0) 0 "DoNotLock" true false)
    (return false)
    (else
      (return false))))

(fn Lookat
  (params (Interactor :type BP%20First%20Person%20Character%20Object%20Reference) (Controller :type Player%20Controller%20Object%20Reference) (HitComponent :type Primitive%20Component%20Object%20Reference))
  (return self HitComponent ""))