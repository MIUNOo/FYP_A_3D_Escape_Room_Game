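; Basic interactable door that swings open once, with an optional locked state.
; Player interaction on an unlocked door calls OnTrigger, which clears the lock and plays a timeline rotating the Door component up to 90 degrees in yaw.
; LookAt supplies a locked or click-to-open prompt.
; There is no closing logic, and the DoorTrigger overlap events only cast to the first-person character without further action.
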(event OnComponentBeginOverlap(DoorTrigger)
  (params (OverlappedComponent :type Primitive%20Component%20Object%20Reference) (OtherActor :type Actor%20Object%20Reference) (OtherComp :type Primitive%20Component%20Object%20Reference) (OtherBodyIndex :type Integer) (bFromSweep :type Boolean) (SweepResult :type Hit%20Result%20Structure%20%28by%20ref%29))
  (Utilities|Casting|CastToBP_FirstPersonCharacter OtherActor))

(event OnComponentEndOverlap(DoorTrigger)
  (params (OverlappedComponent :type Primitive%20Component%20Object%20Reference) (OtherActor :type Actor%20Object%20Reference) (OtherComp :type Primitive%20Component%20Object%20Reference) (OtherBodyIndex :type Integer))
  (Utilities|Casting|CastToBP_FirstPersonCharacter OtherActor))

(event EventBeginPlay
  (Variables|Default|SetIsOpened false))

(event Collision|EventActorBeginOverlap
  (params (OtherActor :type Actor%20Object%20Reference)))

(event EventTick
  (params (DeltaSeconds :type Float%20%28single-precision%29)))

(event EventOnTrigger
  (Variables|Default|SetIsLocked false)
  (if (not (Variables|Default|GetIsOpened))
    (Variables|Default|SetIsOpened true)
    (bind _rotate_door_value (Timeline|OpenDoor PlayFromStart)
      (:Update
        (Transformation|SetRelativeRotation (Variables|Default|GetDoor) (Math|Rotator|MakeRotator 0.0 0.0 (* _rotate_door_value 9e+01)) false false)))))

(fn ConstructionScript)

(fn Interactwith
  (params (Interactor :type BP%20First%20Person%20Character%20Object%20Reference) (HitComponent :type Primitive%20Component%20Object%20Reference))
  (if (Actor|ActorHasTag Interactor "Player")
    (if (not (Variables|Default|GetIsLocked))
      (CallFunction|OnTrigger)
      (return false))))

(fn Lookat
  (params (Interactor :type BP%20First%20Person%20Character%20Object%20Reference) (Controller :type Player%20Controller%20Object%20Reference) (HitComponent :type Primitive%20Component%20Object%20Reference))
  (bind _self self)
  (if (Variables|Default|GetIsLocked)
    (return _self HitComponent "Locked")
    (else
      (return _self HitComponent "Left Click to open door"))))