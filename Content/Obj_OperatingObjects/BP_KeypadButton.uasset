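; BP_KeypadButton is a single clickable key that feeds input to a parent keypad.
; The construction script shows NoText on its Text component.
; A click on Button sends that text and the confirm and return flags to KeypadParent.ButtonClicked, only when the parent can accept entry and is not already entering.
; Without a valid parent, it just prints a placeholder debug string.
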(event OnClicked(Button)
  (params (TouchedComponent :type Primitive%20Component%20Object%20Reference) (ButtonPressed :type Key%20Structure :default "None"))
  (bind _keypadparent (Variables|Default|GetKeypadParent))
  (if (Utilities|IsValid (Variables|Default|GetKeypadParent))
    (if (and (Variables|/Game/Obj_OperatingObjects/BP_Keypad.BP_Keypad_C|GetCan%20Enter _keypadparent) (not (Variables|/Game/Obj_OperatingObjects/BP_Keypad.BP_Keypad_C|GetIs%20Entering _keypadparent)))
      (Default|ButtonClicked (Variables|Default|GetKeypadParent) (Utilities|String|ToString(Text) (Variables|Default|GetNoText)) (Variables|Default|GetIsConfirm) (Variables|Default|GetIsReturn)))
    (else
      (Development|PrintString "Hello"))))

(event EventBeginPlay)

(event Collision|EventActorBeginOverlap
  (params (OtherActor :type Actor%20Object%20Reference)))

(event EventTick
  (params (DeltaSeconds :type Float%20%28single-precision%29)))

(fn ConstructionScript
  (Rendering|Components|TextRender|SetText (Variables|Default|GetText) (Variables|Default|GetNoText)))