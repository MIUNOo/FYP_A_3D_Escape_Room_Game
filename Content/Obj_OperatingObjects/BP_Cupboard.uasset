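; Interactable cupboard with separately lockable top and bottom door pairs and a hidden middle drawer.
; InteractWith checks the interactor's inventory for the matching key, then unlocks by disabling that lock's collision; it does not move the doors itself.
; LookAt returns a locked or interact prompt for the targeted section.
; OnTrigger plays a timeline that slides the drawer along its right vector from the position cached at BeginPlay.
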(event EventBeginPlay
  (Utilities|FlowControl|Sequence
    (:then_0
      (if (not (Variables|Default|GetIsBotLocked))
        (Collision|SetCollisionEnabled (Variables|Default|GetBotLock) "NoCollision")))
    (:then_1
      (if (not (Variables|Default|GetIsTopLocked))
        (Collision|SetCollisionEnabled (Variables|Default|GetTopLock) "NoCollision")))
    (:then_2
      (Variables|Default|SetOriginCaseLocationVec (Transformation|GetWorldLocation (Variables|Default|GetCupboardMidDrawer))))))

(event EventOnTrigger
  (bind _opendrawer (Timeline|Trigger%20hidden Play)
    (:Update
      (Transformation|SetWorldLocation (Variables|Default|GetCupboardMidDrawer) (+ (* (Math|Float|Lerp 0.0 3e+01 _opendrawer) (Math|Vector|GetRightVector (Variables|Default|GetCupboardMidDrawer))) (Variables|Default|GetOriginCaseLocationVec)) true false))))

(fn ConstructionScript)

(fn Interactwith
  (params (Interactor :type BP%20First%20Person%20Character%20Object%20Reference) (HitComponent :type Primitive%20Component%20Object%20Reference))
  (if (Math|Boolean|ORBoolean (== HitComponent (Variables|Default|GetCupboardDoorTL)) (== HitComponent (Variables|Default|GetCupboardDoorTR)) (== HitComponent (Variables|Default|GetTopLock)))
    (if (Variables|Default|GetIsTopLocked)
      (bind _returnvalue (CallFunction|CheckKeyInventory Interactor (Variables|Default|GetKeyforTopLock)))
      (if _returnvalue
        (Variables|Default|SetIsTopLocked false)
        (Collision|SetCollisionEnabled (Variables|Default|GetTopLock) "NoCollision")
        (else
          (return false))))
    (elif (Math|Boolean|ORBoolean (== HitComponent (Variables|Default|GetBotLock)) (== HitComponent (Variables|Default|GetCupboardDoorBL)) (== HitComponent (Variables|Default|GetCupboardDoorBR)))
      (if (Variables|Default|GetIsBotLocked)
        (bind _returnvalue_2 (CallFunction|CheckKeyInventory Interactor (Variables|Default|GetKeyforBotLock)))
        (if _returnvalue_2
          (Variables|Default|SetIsBotLocked false)
          (Collision|SetCollisionEnabled (Variables|Default|GetBotLock) "NoCollision")
          (else
            (return false))))
      (else
        (return false))))
  (return true))

(fn Lookat
  (params (Interactor :type BP%20First%20Person%20Character%20Object%20Reference) (Controller :type Player%20Controller%20Object%20Reference) (HitComponent :type Primitive%20Component%20Object%20Reference))
  (bind _self self)
  (if (Math|Boolean|ORBoolean (== HitComponent (Variables|Default|GetCupboardDoorTL)) (== HitComponent (Variables|Default|GetCupboardDoorTR)) (== HitComponent (Variables|Default|GetTopLock)))
    (if (Variables|Default|GetIsTopLocked)
      _
      (else
        (return _self HitComponent "Left Click to interact with")))
    (elif (Math|Boolean|ORBoolean (== HitComponent (Variables|Default|GetBotLock)) (== HitComponent (Variables|Default|GetCupboardDoorBL)) (== HitComponent (Variables|Default|GetCupboardDoorBR)))
      (if (Variables|Default|GetIsBotLocked)
        _
        (else
          (return _self HitComponent "Left Click to interact with")))
      (else
        (return _self HitComponent ""))))
  (return _self HitComponent "Locked"))