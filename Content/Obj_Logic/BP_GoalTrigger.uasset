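; BP_GoalTrigger is a level goal actor that shows the clear menu when the player reaches it.
; On actor overlap with player 0's character, it creates WB_ClearMenu and adds it to the viewport.
; It then switches to UI-only input with a visible cursor, pauses the game and destroys the player character.
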(event EventBeginPlay)

(event EventTick
  (params (DeltaSeconds :type Float%20%28single-precision%29)))

(event Collision|EventActorBeginOverlap
  (params (OtherActor :type Actor%20Object%20Reference))
  (bind _returnvalue (Game|GetPlayerController 0))
  (if (== OtherActor (Game|GetPlayerCharacter 0))
    (bind _returnvalue_2 (Game|ConstructObjectfromClass "/Game/UIWidget/WB_ClearMenu.WB_ClearMenu_C"))
    (UserInterface|Viewport|AddtoViewport _returnvalue_2 0)
    (Input|SetInputModeUIOnly _returnvalue 0 "DoNotLock" false)
    (Variables|/Script/Engine.PlayerController|SetbShowMouseCursor _returnvalue true)
    (Game|SetGamePaused true)
    (Actor|DestroyActor (Game|GetPlayerCharacter 0))))

(fn ConstructionScript)