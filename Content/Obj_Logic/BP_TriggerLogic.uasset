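; BP_TriggerLogic is a level-editor-placeable trigger that fires a target object when a specific Key actor enters its box.
; IGLE property changes set the Key and TriggerObject references and the SnapKeyToCentre flag.
; On Key overlap it calls OnTrigger through BPI_TriggerObject, optionally teleporting the Key to the trigger's actor location and disabling its physics.
; Its cube is visible and collidable only in level editor mode.
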(event OnComponentBeginOverlap(BoxTrigger)
  (params (OverlappedComponent :type Primitive%20Component%20Object%20Reference) (OtherActor :type Actor%20Object%20Reference) (OtherComp :type Primitive%20Component%20Object%20Reference) (OtherBodyIndex :type Integer) (bFromSweep :type Boolean) (SweepResult :type Hit%20Result%20Structure%20%28by%20ref%29))
  (bind _key (Variables|Default|GetKey))
  (if (and (Utilities|IsValid (Variables|Default|GetTriggerObject)) (Utilities|IsValid (Variables|Default|GetKey)))
    (if (== OtherActor _key)
      (bind _asbpi_trigger_object (Utilities|Casting|CastToBPI_TriggerObject (Variables|Default|GetTriggerObject)))
      (Default|OnTrigger _asbpi_trigger_object)
      (if (Variables|Default|GetSnapKeyToCentre)
        (Transformation|SetActorRelativeTransform _key (Math|Transform|MakeTransform (Transformation|GetActorLocation self) "0, 0, 0" (.scale (Transformation|GetActorTransform _key))) false true)
        (bind _asprimitive_component (Utilities|Casting|CastToPrimitiveComponent (Variables|/Script/Engine.Actor|GetRootComponent _key)))
        (Physics|SetSimulatePhysics _asprimitive_component false)))))

(event OnPropertyValueChanged(IGLE_Interface)
  (params (PropertyName :type String))
  (bind _igle_interface (Variables|Default|GetIGLE_Interface))
  (bind _value (Class|IGLEInterfaceComponent|GetPropertyValuebyName _igle_interface PropertyName))
  (bind _asigle_placable_reference_property_value_object (Utilities|Casting|CastToIGLE_PlacableReferencePropertyValueObject _value)
    (:then
      (switch string PropertyName
        (:Key
          (Variables|Default|SetKey (Class|IGLEFL|IGLEGetActorReference (Variables|/InGameLevelEditor/Properties/PlacableReferenceProperty/IGLE_PlacableReferencePropertyValueObject.IGLE_PlacableReferencePropertyValueObject_C|GetPlacableReference _asigle_placable_reference_property_value_object))))
        (:TriggerObject
          (Variables|Default|SetTriggerObject (Class|IGLEFL|IGLEGetActorReference (Variables|/InGameLevelEditor/Properties/PlacableReferenceProperty/IGLE_PlacableReferencePropertyValueObject.IGLE_PlacableReferencePropertyValueObject_C|GetPlacableReference _asigle_placable_reference_property_value_object))))))
    (:CastFailed
      (bind _asbp_bool_property (Utilities|Casting|CastToBP_BoolProperty _value))
      (if (Utilities|Enum|Equal(Enum) PropertyName "SnapKeyToCentre")
        (Variables|Default|SetSnapKeyToCentre (Variables|/Game/IGE_Maps/BP_BoolProperty.BP_BoolProperty_C|GetValue _asbp_bool_property))))))

(event EventBeginPlay
  (bind _returnvalue (Subsystems|GetIGLERuntimeSubsystem))
  (bind _isinleveleditormode (Variables|/Script/InGameLevelEditor.IGLE_RuntimeSubsystem|GetIsInLevelEditorMode _returnvalue))
  (Development|SetHiddeninGame (Variables|Default|GetCube) (not _isinleveleditormode) false)
  (Collision|SetCollisionEnabled (Variables|Default|GetCube) (select _isinleveleditormode "QueryAndPhysics" (Utilities|Enum|LiteralenumECollisionEnabled "NoCollision"))))

(fn ConstructionScript)