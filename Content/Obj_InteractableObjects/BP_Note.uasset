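; BP_Note is an interactable note that shows a "LMB to read Note" prompt and, when used, opens a WB_Letter widget filled with its NoteContent text.
; While reading, it disables the interactor's movement and look input, hides the HUD and shows the cursor.
; It binds to a CloseWidget event on the player controller's message component, which removes the widget, restores walking, HUD and game input, then unbinds.
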(event Custom|BindEvents
  (bind _ac (Class|BPILockInterface|GetActorComponent(Message) (Game|GetPlayerController 0)))
  (EventDispatchers|BindEventtoCloseWidget _ac (delegate Custom|CloseWidget)))

(event Custom|CloseWidget
  (bind _returnvalue (Game|GetPlayerController 0))
  (bind _interactor (Variables|Default|GetInteractor))
  (Widget|RemovefromParent (Variables|Default|GetLetterWidget))
  (Pawn|Components|CharacterMovement|SetMovementMode (Variables|/Script/Engine.Character|GetCharacterMovement _interactor) "MOVE_Walking" 0)
  (Widget|SetVisibility (Variables|/Game/FirstPerson/Blueprints/BP_FirstPersonCharacter.BP_FirstPersonCharacter_C|GetHeadsUpDisplay _interactor) "Visible")
  (bind _output_get (Variables|/Script/Engine.PlayerController|SetbShowMouseCursor _returnvalue false))
  (bind _output_get_2 (Variables|/Script/Engine.PlayerController|SetbEnableClickEvents _returnvalue _output_get))
  (bind _output_get_3 (Variables|/Script/Engine.PlayerController|SetbEnableMouseOverEvents _returnvalue _output_get_2))
  (Input|SetIgnoreLookInput _returnvalue _output_get_3)
  (Input|SetInputModeGameOnly _returnvalue false)
  (Variables|Default|SetLetterWidget 0)
  (CallFunction|UnbindEvents))

(event Custom|UnbindEvents
  (bind _ac (Class|BPILockInterface|GetActorComponent(Message) (Game|GetPlayerController 0)))
  (EventDispatchers|UnbindallEventsfromCloseWidget _ac))

(event EventBeginPlay)

(event Collision|EventActorBeginOverlap
  (params (OtherActor :type Actor%20Object%20Reference)))

(event EventTick
  (params (DeltaSeconds :type Float%20%28single-precision%29)))

(fn ConstructionScript)

(fn Interactwith
  (params (Interactor :type BP%20First%20Person%20Character%20Object%20Reference) (HitComponent :type Primitive%20Component%20Object%20Reference))
  (bind _returnvalue (Game|GetPlayerController 0))
  (Utilities|IsValid (Variables|Default|GetLetterWidget)
    (:Is%20Not%20Valid
      (CallFunction|BindEvents)
      (bind _returnvalue_2 (UserInterface|CreateWidget "/Game/FirstPerson/WB_Letter.WB_Letter_C"))
      (bind _output_get (Variables|Default|SetLetterWidget _returnvalue_2))
      (Variables|/Script/UMG.TextBlock|SetText (Variables|/Game/FirstPerson/WB_Letter.WB_Letter_C|GetContent _output_get) (Utilities|Text|ToText(String) (Variables|Default|GetNoteContent)))
      (UserInterface|Viewport|AddtoViewport _output_get 0)
      (bind _output_get_2 (Variables|Default|SetInteractor Interactor))
      (Pawn|Components|CharacterMovement|DisableMovement (Variables|/Script/Engine.Character|GetCharacterMovement _output_get_2))
      (Widget|SetVisibility (Variables|/Game/FirstPerson/Blueprints/BP_FirstPersonCharacter.BP_FirstPersonCharacter_C|GetHeadsUpDisplay _output_get_2) "Hidden")
      (bind _output_get_3 (Variables|/Script/Engine.PlayerController|SetbShowMouseCursor _returnvalue true))
      (bind _output_get_4 (Variables|/Script/Engine.PlayerController|SetbEnableClickEvents _returnvalue _output_get_3))
      (Variables|/Script/Engine.PlayerController|SetbEnableMouseOverEvents _returnvalue _output_get_4)
      (Input|SetInputModeGameandUI _returnvalue 0 "DoNotLock" true false)
      (Input|SetIgnoreLookInput _returnvalue true)
      (return false))))

(fn Lookat
  (params (Interactor :type BP%20First%20Person%20Character%20Object%20Reference) (Controller :type Player%20Controller%20Object%20Reference) (HitComponent :type Primitive%20Component%20Object%20Reference))
  (return self HitComponent "LMB to read Note"))