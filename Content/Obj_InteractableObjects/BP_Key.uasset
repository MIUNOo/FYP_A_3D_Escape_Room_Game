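; BP_Key is an interactable key pickup that the player can collect into a key inventory.
; Its mesh simulates physics from BeginPlay, except when the IGLE runtime subsystem reports level editor mode.
; LookAt supplies the pickup prompt, and InteractWith adds the key actor itself to the interactor's KeyInventory.
; Pickup disables the mesh's physics, collision, shadow and visibility instead of destroying the actor, so the inventory reference stays valid.
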(event EventBeginPlay
  (Physics|SetSimulatePhysics (Variables|Default|GetKey) (not (Variables|/Script/InGameLevelEditor.IGLE_RuntimeSubsystem|GetIsInLevelEditorMode (Subsystems|GetIGLERuntimeSubsystem)))))

(event Collision|EventActorBeginOverlap
  (params (OtherActor :type Actor%20Object%20Reference)))

(event EventTick
  (params (DeltaSeconds :type Float%20%28single-precision%29)))

(fn ConstructionScript)

(fn Interactwith
  (params (Interactor :type BP%20First%20Person%20Character%20Object%20Reference) (HitComponent :type Primitive%20Component%20Object%20Reference))
  (bind _output_get (Variables|/Game/FirstPerson/Blueprints/BP_FirstPersonCharacter.BP_FirstPersonCharacter_C|SetKeyInventory Interactor (Variables|/Game/FirstPerson/Blueprints/BP_FirstPersonCharacter.BP_FirstPersonCharacter_C|GetKeyInventory Interactor)))
  (Utilities|Array|Add _output_get self)
  (Physics|SetSimulatePhysics (Variables|Default|GetKey) false)
  (Collision|SetCollisionEnabled (Variables|Default|GetKey) "NoCollision")
  (Rendering|SetCastShadow (Variables|Default|GetKey) false)
  (Rendering|SetVisibility (Variables|Default|GetKey) false false)
  (return false))

(fn Lookat
  (params (Interactor :type BP%20First%20Person%20Character%20Object%20Reference) (Controller :type Player%20Controller%20Object%20Reference) (HitComponent :type Primitive%20Component%20Object%20Reference))
  (return self HitComponent "Left click to pick up"))