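; BP_GreenApple is an interactable green apple prop that identifies itself as "Apple" when looked at.
; On BeginPlay it applies its SimulatePhysics variable to the GreenApple component.
; InteractWith only returns that same flag, and LookAt returns the actor, the hit component and the label.
; Tick is empty, and two swept AddActorWorldTransform nudges are left unconnected.
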(event EventBeginPlay
  (Physics|SetSimulatePhysics (Variables|Default|GetGreenApple) (Variables|Basic|GetSimulatePhysics)))

(event Collision|EventActorBeginOverlap
  (params (OtherActor :type Actor%20Object%20Reference)))

(event EventTick
  (params (DeltaSeconds :type Float%20%28single-precision%29)))

(fn ConstructionScript)

(fn Interactwith
  (params (Interactor :type BP%20First%20Person%20Character%20Object%20Reference) (HitComponent :type Primitive%20Component%20Object%20Reference))
  (return (Variables|Basic|GetSimulatePhysics)))

(fn Lookat
  (params (Interactor :type BP%20First%20Person%20Character%20Object%20Reference) (Controller :type Player%20Controller%20Object%20Reference) (HitComponent :type Primitive%20Component%20Object%20Reference))
  (return self HitComponent "Apple"))