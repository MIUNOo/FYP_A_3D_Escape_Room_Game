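; BP_StaticMeshClass is a static mesh level object with configurable physics simulation and an option to start hidden.
; Hidden objects bind to the appear and vanish events of the player controller's actor component message.
; Those events toggle visibility and collision, turning physics off while hidden and restoring the configured setting on appearance.
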(event Custom|Bind%20Events
  (bind _ac (Class|BPILockInterface|GetActorComponent(Message) (Game|GetPlayerController 0)))
  (EventDispatchers|BindEventtoObjectAppear _ac (delegate Custom|ShowObject))
  (EventDispatchers|BindEventtoObjectVanish _ac (delegate Custom|HideObject)))

(event Custom|ShowObject
  (Physics|SetSimulatePhysics (Variables|Default|GetStaticMesh) (Variables|Default|GetSimulatePhysics))
  (Rendering|SetActorHiddenInGame false)
  (Collision|SetActorEnableCollision true))

(event Custom|HideObject
  (Physics|SetSimulatePhysics (Variables|Default|GetStaticMesh) false)
  (Rendering|SetActorHiddenInGame true)
  (Collision|SetActorEnableCollision false))

(event EventBeginPlay
  (Physics|SetSimulatePhysics (Variables|Default|GetStaticMesh) (Variables|Default|GetSimulatePhysics))
  (if (Variables|Default|GetIsHiddenObject)
    (CallFunction|HideObject)
    (CallFunction|BindEvents)))

(fn ConstructionScript)